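; Map constructor actor that generates a grid level of immortal and destructible walls.
; BuildMapGeometry destroys the actors in MapGeometryArray, then spawns immortal walls on edges and odd-odd cells and destructible walls elsewhere by probability, adding each to the array.
; Cells listed in IdxsToAvoid stay empty.
; BeginPlay and the construction script are empty; a child-actor-component version of the layout sits unconnected in the construction script.
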(event Custom|Build%20Map%20Geometry
  (bind _num_columns (Variables|Default|GetNum%20Columns))
  (bind _num_rows (Variables|Default|GetNum%20Rows))
  (bind _returnvalue (- _num_columns 1))
  (bind _returnvalue_2 (- _num_rows 1))
  (for _array_element (Variables|Default|GetMap%20Geometry%20Array)
    (Actor|DestroyActor _array_element))
  (for _index (range 0 _returnvalue)
    (for _index_2 (range 0 _returnvalue_2)
      ;[1 1 1] Do not spawn anything on indexes to avoid
      (if (not (Utilities|Array|ContainsItem (Variables|Default|GetIdxs%20To%20Avoid) (Math|Vector2D|MakeVector2D (Math|Conversions|ToFloat(Integer) _index_2) (Math|Conversions|ToFloat(Integer) _index))))
        (if (Math|Boolean|ORBoolean (and (> (Math|Integer|%(Integer) _index 2) 0) (> (Math|Integer|%(Integer) _index_2 2) 0)) (or (== _index 0) (== _index _returnvalue)) (or (== _index_2 0) (== _index_2 _returnvalue_2)))
          (bind _returnvalue_3 (Game|SpawnActorfromClass "/Game/Blueprints/MapConstruction/ImmortalWall.ImmortalWall_C" (Math|Transform|MakeTransform (+ (Transformation|GetActorLocation) (Math|Vector|MakeVector (* _index_2 (Variables|Default|GetOffset)) (* _index (Variables|Default|GetOffset)) (.z (Transformation|GetActorLocation)))) "0, 0, 0" "1,1,1") "Undefined" 0 0))
          (Utilities|Array|Add (Variables|Default|GetMap%20Geometry%20Array) _returnvalue_3)
          (else
            ;[1 1 1] Spawn Destructible Wall by probability
            (bind _is_picked (CallFunction|PickItembyProbability (Variables|Default|GetDestructible%20Wall%20Chance)))
            (if _is_picked
              (bind _returnvalue_4 (Game|SpawnActorfromClass "/Game/Blueprints/MapConstruction/DestructibleWall.DestructibleWall_C" (Math|Transform|MakeTransform (+ (Transformation|GetActorLocation) (Math|Vector|MakeVector (* _index_2 (Variables|Default|GetOffset)) (* _index (Variables|Default|GetOffset)) (.z (Transformation|GetActorLocation)))) "0, 0, 0" "1,1,1") "Undefined" 0 0))
              (Utilities|Array|Add (Variables|Default|GetMap%20Geometry%20Array) _returnvalue_4))))))))

(event EventBeginPlay)

(fn ConstructionScript)