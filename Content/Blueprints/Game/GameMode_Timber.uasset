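; Game mode for the Timber game that shows a start screen and sets up local multiplayer.
; On BeginPlay it adds the start screen widget to the viewport, then creates local players 1 to 3 alongside the default player.
; A disconnected branch in the spawn function would spawn and possess a Timber character per player, but it never runs.
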(event EventBeginPlay
  (bind _returnvalue (UserInterface|CreateWidget "/Game/Widgets/StartScreenWidget.StartScreenWidget_C"))
  (UserInterface|Viewport|AddtoViewport _returnvalue 0)
  (CallFunction|FnSpawnPlayers))

(event EventTick
  (params (DeltaSeconds :type Float%20%28single-precision%29)))

(fn ConstructionScript)

(fn FnSpawnPlayers
  (for _index (range 1 3)
    (Class|GameplayStatics|CreatePlayer _index)))