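; Player character for Timber with a sprite, spawned at the PlayerStart tagged with its player number, which its text label also shows.
; Movement input repositions an EndPoint that aims the Fire line trace, which tilts a hit BP_Tree through a timeline or destroys a DestructibleWall.
; Speed pickups raise walk speed until a timer restores a fixed default.
; Sprite-facing and flipbook logic exists but is never triggered here.
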(event Custom|UpdateAnimation
  (bind _sprite (Variables|Default|GetSprite))
  (bind _sprite_2 (Variables|Default|GetSprite))
  ;[1 1 1] Update Sprite Direction and Animation
  (Math|Float|CompareFloat (.x (Variables|/Script/Engine.MovementComponent|GetVelocity (Variables|Character|GetCharacterMovement))) 0.0
    (:>
      (Transformation|SetRelativeRotation _sprite (Math|Rotator|MakeRotator 9e+01 0.0 0.0) false false))
    (:==
      (Math|Float|CompareFloat (.y (Variables|/Script/Engine.MovementComponent|GetVelocity (Variables|Character|GetCharacterMovement))) 0.0
        (:>
          (Transformation|SetRelativeRotation _sprite_2 (Math|Rotator|MakeRotator 9e+01 0.0 0.0) false false))
        (:<
          (Transformation|SetRelativeRotation _sprite_2 (Math|Rotator|MakeRotator -9e+01 0.0 1.8e+02) false false))))
    (:<
      (Transformation|SetRelativeRotation _sprite (Math|Rotator|MakeRotator -9e+01 0.0 1.8e+02) false false))))

(event EventBeginPlay
  (Utilities|IsValid (Variables|references|GetGameState_Ref)
    (:Is%20Valid
      _)
    (:Is%20Not%20Valid
      (Variables|references|SetGameState_Ref (.AsGame%20State%20Timber (Utilities|Casting|CastToGameState_Timber (Game|GetGameState))))))
  (CallFunction|FnSpawn))

(event Collision|EventActorBeginOverlap
  (params (OtherActor :type Actor%20Object%20Reference)))

(event EventTick
  (params (DeltaSeconds :type Float%20%28single-precision%29)))

(event EventPickUpPickup
  (params (Pickup :type Pickup%20Base%20Object%20Reference))
  (bind _charactermovement (Variables|Character|GetCharacterMovement))
  (bind _asspeedup_run_pickup (Utilities|Casting|CastToSpeedupRun_Pickup Pickup))
  (bind _returnvalue (Utilities|Time|SetTimerbyFunctionName 0 "fnSpeedUpEnd" (Variables|/Game/Blueprints/Pickups/SpeedupRun_Pickup.SpeedupRun_Pickup_C|GetSpeedup%20Action%20Time _asspeedup_run_pickup)))
  (Variables|Default|SetSpeedupTimer _returnvalue)
  (Variables|/Script/Engine.CharacterMovementComponent|SetMaxWalkSpeed _charactermovement (+ (Variables|/Script/Engine.CharacterMovementComponent|GetMaxWalkSpeed _charactermovement) (Variables|/Game/Blueprints/Pickups/SpeedupRun_Pickup.SpeedupRun_Pickup_C|GetAdditional%20Speed _asspeedup_run_pickup)))
  (Actor|DestroyActor _asspeedup_run_pickup))

(event Input|ActionEvents|InputActionFire
  (params (Key :type Key%20Structure :default "AnyKey"))
  (bind _self self)
  (:Pressed
    (bind (_outhit _returnvalue) (Collision|LineTraceByChannel (Transformation|GetActorLocation _self) (Transformation|GetWorldLocation (Variables|Default|GetEndPoint _self)) "TraceTypeQuery1" false 0 "Persistent"))
    (if _returnvalue
      (if (.bSuccess (Utilities|Casting|CastToBP_Tree (.HitActor (Collision|BreakHitResult _outhit))))
        (Development|PrintString (Utilities|String|ToString(Vector) (Math|Vector|Normalize (- (Transformation|GetActorLocation self) (.TraceEnd (Collision|BreakHitResult _outhit))))))
        ;[1 1 1] HIT Tree
        (bind _rotationalpha (Timeline|Timeline_0 PlayFromStart)
          (:Update
            (Transformation|SetActorRotation (.AsBP%20Tree (Utilities|Casting|CastToBP_Tree (.HitActor (Collision|BreakHitResult _outhit)))) (Math|Rotator|MakeRotator (* _rotationalpha (.y (Math|Vector|Normalize (- (Transformation|GetActorLocation self) (.TraceEnd (Collision|BreakHitResult _outhit))))) 1.0) (* _rotationalpha (.x (Math|Vector|Normalize (- (Transformation|GetActorLocation self) (.TraceEnd (Collision|BreakHitResult _outhit))))) -1.0) 0.0))))
        (else
          ;[1 1 1] DesdtructibleBlock
          (if (.bSuccess (Utilities|Casting|CastToDestructibleWall (.HitActor (Collision|BreakHitResult _outhit))))
            (Actor|DestroyActor (.AsDestructible%20Wall (Utilities|Casting|CastToDestructibleWall (.HitActor (Collision|BreakHitResult _outhit)))))))))))

(event Input|AxisEvents|InputAxisMove_Right
  (params (AxisValue :type Float%20%28single-precision%29))
  (Pawn|Input|AddMovementInput "0.000000,1.000000, 0" AxisValue false)
  (CallFunction|FnCharTurn (Math|Float|Ceil AxisValue)))

(event Input|AxisEvents|InputAxisMove_Up
  (params (AxisValue :type Float%20%28single-precision%29))
  (Pawn|Input|AddMovementInput "1.000000,0.000000, 0" AxisValue false)
  (CallFunction|FnCharTurn 0 (Math|Float|Ceil AxisValue)))

(fn ConstructionScript)

(fn FnSpawn
  (bind _playerint (Variables|Default|GetPlayerInt))
  (bind _returnvalue (Utilities|String|ToString(Integer) _playerint))
  (bind _returnvalue_2 (Utilities|String|Append "Player" _returnvalue))
  (bind _outactors (Actor|GetAllActorsOfClass "/Script/Engine.PlayerStart"))
  (for _array_element _outactors
    (if (Utilities|Name|Equal(Name) (Variables|/Script/Engine.PlayerStart|GetPlayerStartTag _array_element) (Utilities|String|StringToName _returnvalue_2))
      (bind _output_get (Variables|Default|SetSpawnLocation (Transformation|GetActorTransform _array_element)))
      (Transformation|SetActorTransform _output_get)
      (Rendering|Components|TextRender|SetText (Variables|Default|GetTextRender) (Utilities|Text|ToText(String) _returnvalue_2)))))

(fn FnCharTurn
  (params (x :type Integer) (y :type Integer))
  (if (or (!= x 0) (!= y 0))
    (Transformation|SetRelativeTransform (Variables|Default|GetEndPoint) (Math|Transform|MakeTransform (Math|Vector|MakeVector (Math|Conversions|ToFloat(Integer) (* x -100)) (Math|Conversions|ToFloat(Integer) (* y 100)) 0.0) (Math|Rotator|MakeRotator 0.0 0.0 0.0) "1,1,1") false false)))

(fn FnSpeedUpEnd
  (Variables|/Script/Engine.CharacterMovementComponent|SetMaxWalkSpeed (Variables|Character|GetCharacterMovement) 6e+02)
  (Utilities|Time|ClearandInvalidateTimerbyHandle (Variables|Default|GetSpeedupTimer))
  (Development|PrintString "END"))