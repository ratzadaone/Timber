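; DummyPawn is a placeholder pawn that swaps itself for a playable Timber character when its player presses Fire, apparently as a local multiplayer join step.
; The press reads the controller ID from PlayerController_Timber, calls CreatePlayer with it and spawns PlayerChar_Timber at a fixed elevated location.
; The player controller at that index possesses the new character, then the dummy destroys itself.
; Debug prints remain in the chain.
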(event EventBeginPlay)

(event Collision|EventActorBeginOverlap
  (params (OtherActor :type Actor%20Object%20Reference)))

(event EventTick
  (params (DeltaSeconds :type Float%20%28single-precision%29)))

(event Input|ActionEvents|InputActionFire
  (params (Key :type Key%20Structure :default "AnyKey"))
  (bind _self self)
  (bind _returnvalue (Pawn|GetController _self))
  (:Pressed
    (Development|PrintString "AAAAAAAAo")
    (Development|PrintString (Utilities|GetObjectName _returnvalue))
    (bind _returnvalue_2 (Class|GameplayStatics|GetPlayerControllerID (.AsPlayer%20Controller%20Timber (Utilities|Casting|CastToPlayerController_Timber _returnvalue))))
    (Development|PrintString (Utilities|String|ToString(Integer) _returnvalue_2))
    (Class|GameplayStatics|CreatePlayer _returnvalue_2)
    (bind _returnvalue_3 (Game|SpawnActorfromClass "/Game/Blueprints/Characters/PlayerChar_Timber.PlayerChar_Timber_C" (Math|Transform|MakeTransform "0, 0,2000.000000") "Undefined" 0 _returnvalue_2 0))
    (Pawn|Possess (Game|GetPlayerController _returnvalue_2) _returnvalue_3)
    (Actor|DestroyActor)))

(fn ConstructionScript)